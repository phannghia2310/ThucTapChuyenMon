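; Melee weapon actor that supplies attack montages and socket transforms and handles its own visual effects and drop physics.
; A dynamic glimmer material drives charge glow, while toggles control blood particles, which leave decals on collision, and a briefly animated skeletal trail.
; Regular and combo montages are indexed by array length modulo attack count (not the reverse), with a separate fixed charge montage.
; Dropping switches the mesh to blocking, simulated physics.
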(event OnParticleCollide(P_Blood)
  (params (EventName :type Name :default "None") (EmitterTime :type Float%20%28single-precision%29) (ParticleTime :type Integer) (Location :type Vector :default "0, 0, 0") (Velocity :type Vector :default "0, 0, 0") (Direction :type Vector :default "0, 0, 0") (Normal :type Vector :default "0, 0, 0") (BoneName :type Name :default "None") (PhysMat :type Physical%20Material%20Object%20Reference))
  ;[0.05127 0.05127 0.05127] Partivle Collide Blood
  (Rendering|Decal|SpawnDecalatLocation "/Game/MSPresets/M_MS_Decal_Material/M_MS_Decal_Material.M_MS_Decal_Material" "10.000000,10.000000,10.000000" Location "-90.000000,0.000000,0.000000" 0.0))

(event EventBeginPlay
  (bind _returnvalue (Rendering|Material|CreateDynamicMaterialInstance (Variables|Default|GetWeapon%20Mesh) 0 "/Game/InfinityBladeWeapons/Weapons/Blade/Swords/Blade_Glimmer/M_Blade_Glimmer.M_Blade_Glimmer" "None" :!class /Script/Engine.PrimitiveComponent))
  (Variables|Default|SetweaponMaterial _returnvalue))

(event Collision|EventActorBeginOverlap
  (params (OtherActor :type Actor%20Object%20Reference)))

(event EventToggleWeaponTrail
  (params (enable :type Boolean))
  (bind _sk_trail (Variables|Default|GetSK_Trail))
  (if enable
    (Components|Animation|PlayAnimation _sk_trail "/Game/MyGame/Particles/Sword/Cube/CubeAnim.CubeAnim" true)
    (Utilities|FlowControl|Delay 0.2)
    (Audio|Components|Audio|Stop _sk_trail)))

(event EventTick
  (params (DeltaSeconds :type Float%20%28single-precision%29)))

(event EventDropWeapon
  (bind _weapon_mesh (Variables|Default|GetWeapon%20Mesh))
  ;[0.05127 0.05127 0.05127] Drop Weapon
  (Collision|SetCollisionEnabled _weapon_mesh "PhysicsOnly")
  (Collision|SetCollisionProfileName _weapon_mesh "BlockAll" true :!class /Script/Engine.PrimitiveComponent)
  (Physics|SetSimulatePhysics _weapon_mesh true))

(event EventToggleChargeWeapon
  (params (enable :type Boolean))
  ;[0.05127 0.05127 0.05127] Charge Weapon
  (Rendering|Material|SetScalarParameterValue (Variables|Default|GetweaponMaterial) "Charge Multiplier" (select enable 5e+01 0.0) :!class /Script/Engine.MaterialInstanceDynamic))

(event EventToggleBloodTrail
  (params (enable :type Boolean))
  (bind _p_blood (Variables|Default|GetP_Blood))
  ;[0.05127 0.05127 0.05127] Toggle Blood Trail
  (if enable
    (Components|Activation|Activate _p_blood true)
    (else
      (Components|Activation|Deactivate _p_blood))))

(fn ConstructionScript)

(fn GetAttackMontage
  (params (attackCount :type Integer) (isComboAttack :type Boolean))
  (bind _regularattacks (Variables|Default|GetregularAttacks))
  (bind _comboattacks (Variables|Default|GetcomboAttacks))
  (if isComboAttack
    (return (Utilities|Array|Get(acopy) _comboattacks (Math|Integer|%(Integer) (Utilities|Array|Length _comboattacks) attackCount)))
    (else
      (return (Utilities|Array|Get(acopy) _regularattacks (Math|Integer|%(Integer) (Utilities|Array|Length _regularattacks) attackCount))))))

(fn GetChargeMontage
  (return "/Game/MyGame/Character/Knight/Sword_Animations/Sword_And_Shield_Slash_Montage_Charge.Sword_And_Shield_Slash_Montage_Charge"))

(fn GetWeaponSocketLocation
  (params (socketName :type Name :default "None"))
  (return (Transformation|GetSocketTransform (Variables|Default|GetWeapon%20Mesh) socketName "RTS_World")))