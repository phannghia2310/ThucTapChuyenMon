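; Player controller Blueprint that toggles the pause menu when the PauseGame input action is pressed.
; Opening creates a WB_PauseMenu widget, adds it to the viewport, switches to UI-only input focused on it, shows the cursor and pauses the game.
; Closing removes and clears the widget, restores game-only input, hides the cursor and unpauses.
; An IsPauseMenuOpen flag tracks which branch to run.
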(event EventBeginPlay)

(event EventTick
  (params (DeltaSeconds :type Float%20%28single-precision%29)))

(event Input|ActionEvents|InputActionPauseGame
  (params (Key :type Key%20Structure :default "None"))
  ;[0.05127 0.05127 0.05127] Pause Game
  (:Pressed
    (if (Variables|Default|GetIsPauseMenuOpen)
      (Variables|Default|SetIsPauseMenuOpen false)
      (Widget|RemovefromParent (Variables|Default|GetWB_PauseMenu))
      (Variables|Default|SetWB_PauseMenu 0)
      (Input|SetInputModeGameOnly self)
      (Variables|Default|SetbShowMouseCursor false)
      (Game|SetGamePaused false)
      (else
        (Variables|Default|SetIsPauseMenuOpen true)
        (bind _returnvalue (UserInterface|CreateWidget "/Game/MyGame/Blueprints/UI/WB_PauseMenu.WB_PauseMenu_C" (Game|GetPlayerController 0)))
        (bind _output_get (Variables|Default|SetWB_PauseMenu _returnvalue))
        (UserInterface|Viewport|AddtoViewport _output_get 0)
        (Input|SetInputModeUIOnly self (Variables|Default|GetWB_PauseMenu) "DoNotLock")
        (Variables|Default|SetbShowMouseCursor true)
        (Game|SetGamePaused true)))))

(fn ConstructionScript)